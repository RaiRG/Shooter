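; AI switch actor that toggles behavior trees for every SAIController in the level.
; On BeginPlay it applies its IsEnabled state through ChangeTreeBehavior.
; When an SPlayerCharacter overlaps it, it flips IsEnabled and launches or stops each controller's behavior tree accordingly, with debug prints.
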(event `self.ReceiveBeginPlay`
  (`self.ChangeTreeBehavior` (`self.IsEnabled`)))

(event `self.ReceiveActorBeginOverlap`
  (params (OtherActor :type "Actor Object Reference"))
  (bind _returnvalue (not (`self.IsEnabled`)))
  (cast `SPlayerCharacter` OtherActor)
  (`KismetSystemLibrary.PrintString` "Hello")
  (`self.ChangeTreeBehavior` _returnvalue)
  (set `self.IsEnabled` _returnvalue))

(fn `ChangeTreeBehavior`
  (params (Enable :type Boolean))
  (bind _outactors (`GameplayStatics.GetAllActorsOfClass` "/Script/Shooter.SAIController"))
  (for _array_element _outactors
    (if Enable
      (`SAIController.LaunchBehaviorTree` _array_element)
      (`KismetSystemLibrary.PrintString` "Laucnh")
      (else
        (`SAIController.StopBehaviorTree` _array_element)))))

(fn `UserConstructionScript`)